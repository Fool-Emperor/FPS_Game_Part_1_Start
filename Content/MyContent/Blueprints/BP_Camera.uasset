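; Security camera actor that sweeps back and forth and catches the first-person player when spotted.
; MoveCamera loops on a delay, using a FlipFlop to ease the camera mesh between start and end rotations at a configurable speed.
; Every tick, a forward line trace for pawns runs from the Linetrace component, with debug drawing on.
; A hit on the player sets IsCaught on the character and disables its input.
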(event `self.ReceiveBeginPlay`
  (`|ExecutionSequence`
    (:`then_0`
      ; Setup Player Reference
      (bind _asbp_first_person_character (cast `/Game/MyContent/Blueprints/BP_FirstPersonCharacter` (`GameplayStatics.GetPlayerCharacter` 0)))
      (set `self.PlayerReference` _asbp_first_person_character))
    (:`then_1`
      ; Setup Move Camera
      (`self.MoveCamera`))))

(event `MoveCamera`
  ; Move Camera
  (`/Engine/EditorBlueprintResources/StandardMacros.FlipFlop`
    (:`A`
      (set `self.CurrentRotation` (`self.StartRotation`)))
    (:`B`
      (set `self.CurrentRotation` (`self.EndRotation`))))
  (`KismetSystemLibrary.MoveComponentTo` (`self.SM_Camera`) (0.0 0.0 0.0) (`self.CurrentRotation`) true true (`self.Speed`))
  (`KismetSystemLibrary.Delay` (`self.Delay`))
  (`self.MoveCamera`))

(event `Detect`
  (bind _linetrace (`self.Linetrace`))
  (bind _returnvalue (`SceneComponent.K2_GetComponentLocation` _linetrace))
  ; Detect
  (bind _outhit (`KismetSystemLibrary.LineTraceSingleForObjects` :`Start` _returnvalue :`End` (+ _returnvalue (* (`KismetMathLibrary.GetForwardVector` (`SceneComponent.K2_GetComponentRotation` _linetrace)) (`self.DetectDistance`))) :`ObjectTypes` (`|MakeArray` "ObjectTypeQuery3" :!type "EObjectTypeQuery Enum") :`DrawDebugType` "ForOneFrame"))
  (if (== (`.HitActor` (`GameplayStatics.BreakHitResult` _outhit)) (`self.PlayerReference`))
    (`|ExecutionSequence`
      (:`then_0`
        (set `/Game/MyContent/Blueprints/BP_FirstPersonCharacter.IsCaught` true (`self.PlayerReference`))
        ; Disable Input and Reset Level
        (`self.DisableInput` (`self.PlayerReference`) (`GameplayStatics.GetPlayerController` 0))))))

(event `self.ReceiveTick`
  (params (DeltaSeconds :type "Float (single-precision)"))
  (`self.Detect`))

(fn `UserConstructionScript`)