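; Key-locked door actor that swings open when the player enters its trigger zone holding a key, and swings back when they leave.
; On overlap it checks HasKey on the cached first-person character, and a timeline lerps the door mesh's rotation, reversing on exit.
; A dynamic material instance on the light mesh brightens green for access or red for no key, then returns to dim yellow.
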(event `self.ReceiveBeginPlay`
  ; Set Up Variables
  (`|ExecutionSequence`
    (:`then_0`
      ;;[0.5705 0.8073 0.387 0.5] Set Up Player Character
      (bind _asbp_first_person_character (cast `/Game/MyContent/Blueprints/BP_FirstPersonCharacter` (`GameplayStatics.GetPlayerCharacter` 0)))
      (set `self.PlayerReference` _asbp_first_person_character))
    (:`then_1`
      ;;[0.3566 0.849 0.3494 0.5] Set Up Material Variable
      (bind _returnvalue (`KismetMaterialLibrary.CreateDynamicMaterialInstance` "/Game/MyContent/Materials/MI_Light.MI_Light"))
      (bind _output_get (set `self.DynamicMaterial` _returnvalue))
      (`PrimitiveComponent.SetMaterial` (`self.SM_Light`) 0 _output_get))))

(event `self.Door_TriggerZone.OnComponentBeginOverlap`
  (params (OverlappedComponent :type "PrimitiveComponent Object Reference") (OtherActor :type "Actor Object Reference") (OtherComp :type "PrimitiveComponent Object Reference") (OtherBodyIndex :type Integer) (bFromSweep :type Boolean) (SweepResult :type "HitResult Structure (by ref)"))
  ; Light Change
  (if (== OtherActor (`self.PlayerReference`))
    (`MaterialInstanceDynamic.SetScalarParameterValue` (`self.DynamicMaterial`) "Intensity" 100.0)
    (if (`/Game/MyContent/Blueprints/BP_FirstPersonCharacter.HasKey` (`self.PlayerReference`))
      (`MaterialInstanceDynamic.SetVectorParameterValue` (`self.DynamicMaterial`) "Colour" (struct :`R` 0.14316 :`G` 1.0 :`A` 1.0))
      ; Door Open Close
      (bind (_direction _alpha) (`Timeline|Timeline_DoorOpenClose` :!label _label)
        (:`Update`
          (set `self.DoorOpening` true)
          (`SceneComponent.K2_SetRelativeRotation` (`self.SM_Door`) (`KismetMathLibrary.RLerp` (struct) (struct :`Yaw` 90.0) _alpha) false false))
        (:`Finished`
          (set `self.DoorOpening` false)))
      (else
        (`MaterialInstanceDynamic.SetVectorParameterValue` (`self.DynamicMaterial`) "Colour" (struct :`R` 1.0 :`B` 0.041253 :`A` 1.0))))))

(event `self.Door_TriggerZone.OnComponentEndOverlap`
  (params (OverlappedComponent :type "PrimitiveComponent Object Reference") (OtherActor :type "Actor Object Reference") (OtherComp :type "PrimitiveComponent Object Reference") (OtherBodyIndex :type Integer))
  ; Return to Default
  (if (== OtherActor (`self.PlayerReference`))
    (`MaterialInstanceDynamic.SetScalarParameterValue` (`self.DynamicMaterial`) "Intensity" 1.0)
    (`MaterialInstanceDynamic.SetVectorParameterValue` (`self.DynamicMaterial`) "Colour" (struct :`R` 0.428037 :`G` 0.432292 :`B` 0.075685 :`A` 1.0))
    (goto _label :!via `Reverse`)))

(fn `UserConstructionScript`)