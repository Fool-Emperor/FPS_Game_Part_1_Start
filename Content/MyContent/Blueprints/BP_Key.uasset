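; BP_Key is a key pickup that appears once no BP_Target actors remain in the level.
; Each Tick it counts targets through the index returned by an array Add, prints that number, and sets root visibility and actor collision accordingly.
; A DoOnce plays a particle and sound on appearance.
; When the player character overlaps the capsule, it sets HasKey on that character, plays a collect sound and destroys itself.
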(event `self.ReceiveBeginPlay`
  ;[0.651 0 0.2059 0.5] Setup Variables
  (bind _asbp_first_person_character (cast `/Game/MyContent/Blueprints/BP_FirstPersonCharacter` (`GameplayStatics.GetPlayerCharacter` 0)))
  (set `self.PlayerReference` _asbp_first_person_character))

(event `self.ReceiveTick`
  (params (DeltaSeconds :type "Float (single-precision)"))
  (bind _returnvalue (`SceneComponent.K2_GetComponentLocation` (`self.DefaultSceneRoot`)))
  ;[0.1228 0.9826 0.828 0.5] Key - Visibility
  (bind _outactors (`GameplayStatics.GetAllActorsOfClass` "/Game/MyContent/Blueprints/BP_Target.BP_Target_C"))
  (bind _returnvalue_2 (`KismetArrayLibrary.Array_Add` _outactors))
  (`|ExecutionSequence`
    (:`then_0`
      (bind _returnvalue_3 (<= _returnvalue_2 0))
      (`SceneComponent.SetVisibility` (`self.DefaultSceneRoot`) _returnvalue_3 false)
      (`self.SetActorEnableCollision` _returnvalue_3)
      ;[0 0.5625 0.4888 0.5] Key - Spawn
      (if _returnvalue_3
        (`/Engine/EditorBlueprintResources/StandardMacros.DoOnce` false
          (:`Completed`
            (`GameplayStatics.SpawnEmitterAtLocation` "/Engine/Tutorial/SubEditors/TutorialAssets/TutorialParticleSystem.TutorialParticleSystem" _returnvalue)
            (`GameplayStatics.PlaySoundAtLocation` "/Game/MyContent/Audio/MP3_Key_Appear.MP3_Key_Appear" _returnvalue (struct) 1.0 1.0 0.0 null null null null)))))
    (:`then_1`
      (`KismetSystemLibrary.PrintString` (`KismetStringLibrary.Conv_IntToString` _returnvalue_2)))))

(event `self.CapsuleCollider.OnComponentBeginOverlap`
  (params (OverlappedComponent :type "PrimitiveComponent Object Reference") (OtherActor :type "Actor Object Reference") (OtherComp :type "PrimitiveComponent Object Reference") (OtherBodyIndex :type Integer) (bFromSweep :type Boolean) (SweepResult :type "HitResult Structure (by ref)"))
  ;[0 0.9115 0.7364 0.5] Key - Pick Up
  (if (== OtherActor (`self.PlayerReference`))
    (set `/Game/MyContent/Blueprints/BP_FirstPersonCharacter.HasKey` true (`self.PlayerReference`))
    (`GameplayStatics.PlaySoundAtLocation` "/Game/MyContent/Audio/MP3_Key_Collect.MP3_Key_Collect" (`self.K2_GetActorLocation`) (struct) 1.0 1.0 0.0 null null null null)
    (`self.K2_DestroyActor`)))

(fn `UserConstructionScript`)